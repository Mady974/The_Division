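; Capsule actor with an animated mesh and a camera-facing text label, offering a placeholder interaction when the player is nearby.
; A slowed timeline drives the mesh's height and yaw at a fixed tilt, while a delayed FlipFlop on its updates alternates orange and blue materials.
; Tick turns the text toward the player camera.
; Character overlap toggles actor input; overlaps and the Interaction key only print debug messages.
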(event `self.ReceiveActorBeginOverlap`
  (params (OtherActor :type "Actor Object Reference"))
  ;[1 1 1] Enable Input
  (cast `/Game/ThirdPersonBP/Blueprints/ThirdPersonCharacter` OtherActor)
  (`self.EnableInput` (`GameplayStatics.GetPlayerController` 0))
  (`KismetSystemLibrary.PrintString` "U in me "))

(event `self.ReceiveTick`
  (params (DeltaSeconds :type "Float (single-precision)"))
  (bind _textrender (`self.TextRender`))
  ;[1 1 1] Orientation texte
  (`SceneComponent.K2_SetRelativeRotation` _textrender (`KismetMathLibrary.FindLookAtRotation` (`SceneComponent.K2_GetComponentLocation` _textrender) (`SceneComponent.K2_GetComponentLocation` (`self.GetComponentByClass` (`GameplayStatics.GetPlayerCharacter` 0) "/Script/Engine.CameraComponent"))) false false))

(event `InputAction|Interaction`
  (params (Key :type "Key Structure"))
  (:`Pressed`
    (`KismetSystemLibrary.PrintString` "Press Harder")))

(event `self.ReceiveActorEndOverlap`
  (params (OtherActor :type "Actor Object Reference"))
  ;[1 1 1] Enable Input
  (cast `/Game/ThirdPersonBP/Blueprints/ThirdPersonCharacter` OtherActor)
  (`self.DisableInput` (`GameplayStatics.GetPlayerController` 0))
  (`KismetSystemLibrary.PrintString` "Bye cya"))

(event `self.ReceiveBeginPlay`
  ;[1 1 1] Movement and rotation
  (`TimelineComponent.SetPlayRate` (`self.Timeline_0`) 0.25)
  (bind (_direction _movement _rotation) (`Timeline|Timeline_0`)
    (:`Update`
      (`SceneComponent.K2_SetRelativeLocationAndRotation` (`self.StaticMesh`) (`KismetMathLibrary.MakeVector` (.x (`SceneComponent.RelativeLocation` (`self.StaticMesh`))) (.y (`SceneComponent.RelativeLocation` (`self.StaticMesh`))) _movement) (`KismetMathLibrary.MakeRotator` 0.0 -50.0 (* _rotation 360.0)) false false)
      (`KismetSystemLibrary.Delay` 2.0)
      (`/Engine/EditorBlueprintResources/StandardMacros.FlipFlop`
        (:`A`
          (`PrimitiveComponent.SetMaterial` (`self.StaticMesh`) 0 "/Game/TRAORE--BASTIDA/Materials/M_Orange.M_Orange"))
        (:`B`
          (`PrimitiveComponent.SetMaterial` (`self.StaticMesh`) 0 "/Game/TRAORE--BASTIDA/Materials/M_blue.M_blue"))))))

(fn `UserConstructionScript`)